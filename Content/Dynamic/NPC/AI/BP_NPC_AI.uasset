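; AI controller for guard NPCs that runs their behaviour tree and feeds it the currently perceived target.
; On BeginPlay it sets up the BB_PatrolData blackboard and starts BT_GuardBehaviour.
; Perception updates ignore actors tagged "Enemy"; any other sensed actor is written to the EnemyKey blackboard value.
; A failed sense on such an actor clears that key, without checking whether it is the stored target.
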(event `self.ReceiveBeginPlay`
  (bind _blackboardcomponent (`self.UseBlackboard` "/Game/Dynamic/NPC/AI/BB_PatrolData.BB_PatrolData"))
  (set `self.BlackBoardComp` _blackboardcomponent)
  (`self.RunBehaviorTree` "/Game/Dynamic/NPC/AI/BT_GuardBehaviour.BT_GuardBehaviour"))

(event `self.AIPerception.OnTargetPerceptionUpdated`
  (params (Actor :type "Actor Object Reference") (Stimulus :type "AIStimulus Structure"))
  (if (`self.ActorHasTag` Actor "Enemy")
    _
    (elif (`.bSuccessfullySensed` (break `AIStimulus` Stimulus))
      (`BlackboardComponent.SetValueAsObject` (`self.BlackBoardComp`) (`self.EnemyKey`) Actor)
      (else
        (`BlackboardComponent.ClearValue` (`self.BlackBoardComp`) (`self.EnemyKey`))))))

(fn `UserConstructionScript`)